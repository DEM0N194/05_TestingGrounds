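; NPC_AI_BP drives guard NPC AI through a behavior tree, a blackboard and AI perception.
; On BeginPlay it sets up the PatrolData blackboard and runs GuardBehavior.
; Perception updates for actors without the "Enemy" tag store the sensed actor as an object under EnemyLocationKey, or clear that key when sensing fails.
; Actors tagged "Enemy" are ignored.
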(event OnTargetPerceptionUpdated(AIPerception)
  (params (Actor :type Actor%20Object%20Reference) (Stimulus :type AI%20Stimulus%20Structure))
  (bind _blackboardcomp (Variables|Default|GetBlackboardComp))
  (bind _enemylocationkey (Variables|Default|GetEnemyLocationKey))
  (if (not (Actor|ActorHasTag Actor "Enemy"))
    (if (.bSuccessfullySensed (Utilities|Struct|BreakAIStimulus Stimulus))
      (AI|Components|Blackboard|SetValueasObject _blackboardcomp _enemylocationkey Actor)
      (else
        (AI|Components|Blackboard|ClearValue _blackboardcomp _enemylocationkey)))))

(event EventBeginPlay
  (bind _blackboardcomponent (Class|AIController|UseBlackboard "/Game/Dynamic/NPC/AI/PatrolData.PatrolData"))
  (Variables|Default|SetBlackboardComp _blackboardcomponent)
  (AI|RunBehaviorTree "/Game/Dynamic/NPC/AI/GuardBehavior.GuardBehavior"))

(fn ConstructionScript)