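; Terrain tile for an infinite-terrain mode that scatters props, rocks and two AI characters when play begins.
; The player entering the locking volume opens the barrier; leaving it re-locks the barrier, asks the game mode for another tile and reports this one conquered.
; Only the conquest report is guarded against repeats.
; An arrow supplies the attach transform, and player overlap with the destroy volume removes the tile.
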(event OnComponentBeginOverlap(LockingVolume)
  (params (OverlappedComponent :type Primitive%20Component%20Object%20Reference) (OtherActor :type Actor%20Object%20Reference) (OtherComp :type Primitive%20Component%20Object%20Reference) (OtherBodyIndex :type Integer) (bFromSweep :type Boolean) (SweepResult :type Hit%20Result%20Structure%20%28by%20ref%29))
  (Utilities|IsPlayerCharacter OtherActor
    (:True
      (CallFunction|Unlock))))

(event OnComponentEndOverlap(LockingVolume)
  (params (OverlappedComponent :type Primitive%20Component%20Object%20Reference) (OtherActor :type Actor%20Object%20Reference) (OtherComp :type Primitive%20Component%20Object%20Reference) (OtherBodyIndex :type Integer))
  (Utilities|IsPlayerCharacter OtherActor
    (:True
      (CallFunction|Lock)
      (bind _asinfinite_terrain_game_mode (Utilities|Casting|CastToInfiniteTerrainGameMode (Game|GetGameMode)))
      (Default|SpawnTile _asinfinite_terrain_game_mode)
      (CallFunction|TileConquered))))

(event OnComponentBeginOverlap(DestroyVolume)
  (params (OverlappedComponent :type Primitive%20Component%20Object%20Reference) (OtherActor :type Actor%20Object%20Reference) (OtherComp :type Primitive%20Component%20Object%20Reference) (OtherBodyIndex :type Integer) (bFromSweep :type Boolean) (SweepResult :type Hit%20Result%20Structure%20%28by%20ref%29))
  (Utilities|IsPlayerCharacter OtherActor
    (:True
      (Actor|DestroyActor))))

(event EventBeginPlay
  (Class|Tile|PlaceActors "/Game/Dynamic/Terrain/Props/BP_Container.BP_Container_C" (ItemData|MakeSpawnParams 1 3 4e+02 1.0 1.0))
  (Class|Tile|PlaceActors "/Game/Dynamic/Terrain/Props/BP_Box.BP_Box_C" (ItemData|MakeSpawnParams 2 4 1e+02 0.75 1.25))
  (Class|Tile|PlaceActors "/Game/Dynamic/Terrain/Props/BP_Rock_01.BP_Rock_01_C" (ItemData|MakeSpawnParams 1 4 1.5e+02 1.0 5.0))
  (Class|Tile|PlaceActors "/Game/Dynamic/Terrain/Props/BP_Rock_02.BP_Rock_02_C" (ItemData|MakeSpawnParams 1 4 2.5e+02 1.0 5.0))
  (Class|Tile|PlaceActors "/Game/Dynamic/Terrain/Props/BP_Rock_03.BP_Rock_03_C" (ItemData|MakeSpawnParams 1 4 2.5e+02 1.0 5.0))
  (Class|Tile|PlaceActors "/Game/Dynamic/Terrain/Props/BP_SandBags.BP_SandBags_C" (ItemData|MakeSpawnParams 1 2 2.5e+02 1.0 1.0))
  (Class|Tile|PlaceActors "/Game/Dynamic/Terrain/Props/BP_Canister.BP_Canister_C" (ItemData|MakeSpawnParams 1 7 5e+01 1.0 1.0))
  (Class|Tile|PlaceAIPawns "/Game/Dynamic/Character/Behavior/BP_Character.BP_Character_C" (ItemData|MakeSpawnParams 2 2 1e+02 1.0 1.0)))

(event Collision|EventActorBeginOverlap
  (params (OtherActor :type Actor%20Object%20Reference)))

(event EventTick
  (params (DeltaSeconds :type Float%20%28single-precision%29)))

(fn ConstructionScript)

(fn GetAttachLocation
  (return (Transformation|GetWorldTransform (Variables|Default|GetArrow))))

(fn Unlock
  (Collision|SetCollisionEnabled (Variables|Default|GetBarrier) "NoCollision")
  (Rendering|Material|SetMaterial (Variables|Default|GetBarrier) 0 "/Game/Dynamic/Terrain/MI_Barrier_Green.MI_Barrier_Green"))

(fn Lock
  (Collision|SetCollisionEnabled (Variables|Default|GetBarrier) "QueryAndPhysics")
  (Rendering|Material|SetMaterial (Variables|Default|GetBarrier) 0 "/Game/Dynamic/Terrain/MI_Barrier_Red.MI_Barrier_Red"))

(fn TileConquered
  (if (not (Variables|Default|GetConquered))
    (bind _asinfinite_terrain_game_mode (Utilities|Casting|CastToInfiniteTerrainGameMode (Game|GetGameMode)))
    (Default|NewTileConquered _asinfinite_terrain_game_mode)
    (Variables|Default|SetConquered true)))